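; Test actor for runtime content delivery, trying out chunk patching and zip downloads.
; On BeginPlay it loads the cached PatchingDemoLive build, calls UpdateBuild if that fails, and prints results.
; Disconnected experiments cover HTTP archive download, RuntimeArchiver extraction into the Content directory, chunk mounting, and JSON-driven async mesh loading into new components.
; The in-memory unzip handler is bound only from a disconnected download node.
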(event Custom|CustomEvent_0
  (params (BytesReceived :type Integer64) (ContentLength :type Integer64) (ProgressRatio :type Float%20%28single-precision%29))
  (Development|PrintString (Utilities|String|ToString(Float) ProgressRatio)))

(event Custom|CustomEvent_1
  (params (DownloadedContent :type Array%20of%20Bytes) (Result :type EDownloadToMemoryResult%20Enum :default "SuccessDownloading"))
  (bind _returnvalue (Class|KismetSystemLibrary|GetProjectContentDirectory))
  (bind _unarchive_directory_path (Variables|Default|GetUnarchive%20Directory%20Path))
  (bind _array (Utilities|Array|MakeArray _returnvalue _unarchive_directory_path))
  (bind _returnvalue_2 (Class|BlueprintPathsLibrary|Combine _array))
  (bind _outpath (Class|BlueprintPathsLibrary|NormalizeDirectoryName _returnvalue_2))
  (switch Utilities|FlowControl|Switch|SwitchonEDownloadToMemoryResult Result
    (:SuccessDownloading
      (bind _returnvalue_3 (Class|RuntimeArchiverBase|CreateRuntimeArchiver "/Script/RuntimeArchiver.RuntimeArchiverZip"))
      (bind _output_get (Variables|Default|SetRuntimeArchiverRef _returnvalue_3))
      (bind _returnvalue_4 (Class|RuntimeArchiverBase|OpenArchivefromMemory _output_get DownloadedContent))
      (if _returnvalue_4
        (bind (_numofarchiveentries _returnvalue_5) (Class|RuntimeArchiverBase|GetArchiveEntries (Variables|Default|GetRuntimeArchiverRef)))
        (if _returnvalue_5
          (for _index (range 0 _numofarchiveentries)
            (bind (_entryinfo _returnvalue_6) (Class|RuntimeArchiverBase|GetArchiveEntryInfobyIndex (Variables|Default|GetRuntimeArchiverRef) _index))
            (if _returnvalue_6
              (Development|PrintString (.Name (Utilities|Struct|BreakRuntimeArchiveEntry _entryinfo)))
              (Utilities|Array|Add (Variables|Default|GetEntry%20Info) _entryinfo)))
          (Development|PrintString _outpath true true "(R=0.971679,G=1.000000,B=0.000000,A=1.000000)" 5.0)
          (Class|RuntimeArchiverBase|ExtractEntriestoStorage (Variables|Default|GetRuntimeArchiverRef) (delegate Custom|CustomEvent_2) (delegate Custom|CustomEvent_3) (Variables|Default|GetEntry%20Info) _outpath true)
          (else
            (CallFunction|ClearUnrealArchiver)))
        (else
          (CallFunction|ClearUnrealArchiver))))
    (:DownloadFailed
      (Development|PrintString "falid" true true "(R=1.000000,G=0.000000,B=0.000000,A=1.000000)"))))

(event Custom|CustomEvent_2
  (params (bSuccess :type Boolean))
  (Development|PrintString (Utilities|String|ToString(Boolean) bSuccess) true true "(R=1.000000,G=0.058872,B=0.000000,A=1.000000)" 1e+01)
  (if bSuccess
    _))

(event Custom|CustomEvent_3
  (params (Percentage :type Integer)))

(event Custom|OnPatchComplete_Event_0
  (params (Succeeded :type Boolean))
  (Development|PrintString (Utilities|String|ToString(Boolean) Succeeded) true true "(R=1.000000,G=0.000000,B=0.062795,A=1.000000)" 1e+01))

(event Custom|CustomEvent_4
  (params (bWasSuccessful :type Boolean))
  (Development|PrintString (Utilities|String|ToString(Boolean) bWasSuccessful)))

(event Custom|CustomEvent_5
  (params (bWasSuccessful :type Boolean))
  (Development|PrintString (Utilities|String|ToString(Boolean) bWasSuccessful)))

(event Custom|CustomEvent_6
  (params (bWasSuccessful :type Boolean))
  (Development|PrintString (Utilities|String|ToString(Boolean) bWasSuccessful)))

(event EventBeginPlay
  (Utilities|FlowControl|Delay 0.0)
  (bind _returnvalue (Class|ChunkCore|LoadCachedBuild "PatchingDemoLive"))
  (Development|PrintString (Utilities|String|ToString(Boolean) _returnvalue) true true "(R=1.000000,G=0.553727,B=0.000000,A=1.000000)")
  (if (not _returnvalue)
    (Class|ChunkCore|UpdateBuild "PatchingDemoLive" "HttpRequestLive" (delegate Custom|CustomEvent_6))))

(event EventTick
  (params (DeltaSeconds :type Float%20%28single-precision%29)))

(fn ConstructionScript)

(fn ClearUnrealArchiver
  (bind _returnvalue (Class|RuntimeArchiverBase|CloseArchive (Variables|Default|GetRuntimeArchiverRef)))
  (Variables|Default|SetRuntimeArchiverRef 0)
  (return _returnvalue))