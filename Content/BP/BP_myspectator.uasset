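; Spectator Blueprint that serves as a test harness for runtime content patching and async asset loading, with debug prints throughout.
; Left click or first touch async-loads the Loadtest class and spawns it, raising the next spawn point each time.
; Right click or second touch calls PatchGame on MyGameInstance, and Tick then prints download percent.
; A mobile-patching install-and-mount chain and chunk-mount callbacks also exist, but nothing live here starts them.
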(event Custom|CustomEvent_0
  (params (bWasSuccessful :type Boolean))
  (if bWasSuccessful
    (Class|ChunkCore|MountChunk 100 (delegate Custom|CustomEvent_1))
    (else
      (Development|PrintString "falid")
      (Utilities|FlowControl|DoOnce false ; enters at Reset
        (:Completed
          (Class|ChunkCore|BeginLoadingMode (delegate Custom|CustomEvent_0)))))))

(event Custom|CustomEvent_1
  (params (bWasSuccessful :type Boolean))
  (if bWasSuccessful
    (|AsyncLoadPrimaryAssetClass "PrimaryAssetLabel:ChunkB"
      (:Completed
        (Development|PrintString "complite")
        (Variables|Default|SetNewVar_0 true)))
    (else
      (Development|PrintString "falid")
      (Utilities|FlowControl|DoOnce false ; enters at Reset
        (:Completed
          (Class|ChunkCore|BeginLoadingMode (delegate Custom|CustomEvent_0)))))))

(event Custom|DisplayDownloadState
  (params (Target :type Mobile%20Pending%20Content%20Object%20Reference))
  (bind _returnvalue (Class|MobilePendingContent|GetDownloadSize Target))
  ;[1 1 1] Comment
  (Development|PrintText (Utilities|Text|FormatText "{State}: {Percent} Complete. {Reamining} MB of {Total}  MB to download at {Speed} MB/s." (Class|MobilePendingContent|GetDownloadStatusText Target) (Class|KismetTextLibrary|AsPercentFloat (Class|MobilePendingContent|GetInstallProgress Target) "HalfToEven") (- (Class|MobilePendingContent|GetTotalDownloadedSize Target) _returnvalue) _returnvalue (Class|MobilePendingContent|GetDownloadSpeed Target)) true true "(R=1.000000,G=0.000000,B=0.231755,A=1.000000)" 1e+01))

(event Custom|Mount%20Content
  ;[1 1 1] Comment
  (Class|MobileInstalledContent|Mount (Class|MobilePatchingLibrary|GetInstalledContent (Variables|Default|GetInstall%20Directory))))

(event Custom|Patching_Initiated
  ;[1 1 1] Comment
)

(event Custom|OnSucceeded
  (params (MobilePendingContent :type Mobile%20Pending%20Content%20Object%20Reference))
  ;[1 1 1] Comment
  (bind _output_get (Variables|Default|SetMobile%20Pending%20Content MobilePendingContent))
  (CallFunction|CheckDownloadSpace _output_get))

(event Custom|ReqOnFailed
  (params (ErrorText :type Text) (ErrorCode :type Integer))
  ;[1 1 1] Comment
  (Development|PrintString (Utilities|String|ToString(Text) ErrorText) true true "(R=1.000000,G=0.000000,B=0.174660,A=1.000000)" 1e+01))

(event Custom|CheckDownloadSpace
  (params (Mobile%20Pending%20Content :type Mobile%20Pending%20Content%20Object%20Reference))
  ;[1 1 1] Comment
  (if (< (Class|MobilePendingContent|GetRequiredDiskSpace Mobile%20Pending%20Content) (Class|MobileInstalledContent|GetDiskFreeSpace Mobile%20Pending%20Content))
    (CallFunction|StartDownload Mobile%20Pending%20Content)
    (else
      (Development|PrintString "No Space"))))

(event Custom|StartDownload
  (params (Mobile%20Pending%20Content :type Mobile%20Pending%20Content%20Object%20Reference))
  ;[1 1 1] Comment
  (Class|MobilePendingContent|StartInstall Mobile%20Pending%20Content (delegate Custom|InstallOnSuccedded) (delegate Custom|InstallOnFailed))
  (Utilities|Time|SetTimerbyEvent (delegate Custom|UpdateDonwloadState) 0.1 true))

(event Custom|InstallOnSuccedded
  ;[1 1 1] Comment
  (CallFunction|MountContent))

(event Custom|InstallOnFailed
  (params (ErrorText :type Text) (ErrorCode :type Integer))
  ;[1 1 1] Comment
  (Development|PrintString (Utilities|String|ToString(Text) ErrorText)))

(event Custom|UpdateDonwloadState
  ;[1 1 1] Comment
  (CallFunction|DisplayDownloadState (Variables|Default|GetMobile%20Pending%20Content)))

(event EventTick
  (params (DeltaSeconds :type Float%20%28single-precision%29))
  (if (Variables|Default|Getpatching)
    (Development|PrintString (Utilities|String|ToString(Float) (.DownloadPercent (Class|MyGameInstance|GetLoadingProgress (.AsMy%20Game%20Instance (Utilities|Casting|CastToMyGameInstance (Game|GetGameInstance)))))))))

(event Input|KeyboardEvents|C
  (params (Key :type Key%20Structure :default "None")))

(event Input|KeyboardEvents|H
  (params (Key :type Key%20Structure :default "None")))

(event Input|KeyboardEvents|K
  (params (Key :type Key%20Structure :default "None")))

(event Input|MouseEvents|RightMouseButton
  (params (Key :type Key%20Structure :default "None"))
  (:Pressed
    (Development|PrintString "Start Download ")
    (bind _returnvalue (Class|MyGameInstance|PatchGame (.AsMy%20Game%20Instance (Utilities|Casting|CastToMyGameInstance (Game|GetGameInstance)))))
    (Variables|Default|Setpatching true)
    (Development|PrintString (Utilities|String|ToString(Boolean) _returnvalue))))

(event Input|MouseEvents|LeftMouseButton
  (params (Key :type Key%20Structure :default "None"))
  (:Pressed
    (Development|PrintString "spawn")
    (bind _class (Utilities|AsyncLoadClassAsset "/Game/ChunkAssets/files/Loadtest.Loadtest_C")
      (:Completed
        (bind _asactor (Utilities|Casting|CastToActorClass _class))
        (bind _returnvalue (Game|SpawnActorfromClass _asactor (Math|Transform|MakeTransform (Variables|Default|GetLocation)) "Undefined" 0 0))
        (Utilities|IsValid _returnvalue
          (:Is%20Valid
            (bind _output_get (Variables|Default|SetLocation (Math|Vector|MakeVector (.X (Math|Vector|BreakVector (stale _output_get))) (.Y (Math|Vector|BreakVector (stale _output_get))) (+ (.Z (Math|Vector|BreakVector (stale _output_get))) 1.2e+02))))))))))

(event Input|TouchEvents|Touch2
  (params (Key :type Key%20Structure :default "None"))
  (:Pressed
    (Development|PrintString "Start Download ")
    (bind _returnvalue (Class|MyGameInstance|PatchGame (.AsMy%20Game%20Instance (Utilities|Casting|CastToMyGameInstance (Game|GetGameInstance)))))
    (Variables|Default|Setpatching true)
    (Development|PrintString (Utilities|String|ToString(Boolean) _returnvalue))))

(event Input|TouchEvents|Touch1
  (params (Key :type Key%20Structure :default "None"))
  (:Pressed
    (Development|PrintString "spawn")
    (bind _class (Utilities|AsyncLoadClassAsset "/Game/ChunkAssets/files/Loadtest.Loadtest_C")
      (:Completed
        (bind _asactor (Utilities|Casting|CastToActorClass _class))
        (bind _returnvalue (Game|SpawnActorfromClass _asactor (Math|Transform|MakeTransform (Variables|Default|GetLocation)) "Undefined" 0 0))
        (Utilities|IsValid _returnvalue
          (:Is%20Valid
            (bind _output_get (Variables|Default|SetLocation (Math|Vector|MakeVector (.X (Math|Vector|BreakVector (stale _output_get))) (.Y (Math|Vector|BreakVector (stale _output_get))) (+ (.Z (Math|Vector|BreakVector (stale _output_get))) 1.2e+02))))))))))

(fn ConstructionScript)